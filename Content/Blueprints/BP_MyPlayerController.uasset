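; Player controller that owns the in-game HUD and opens minion interaction menus.
; On BeginPlay it creates the IngameUI widget, keeps a reference and adds it to the viewport.
; Minion enter and leave events toggle a hint on that HUD.
; An interact event spawns a new interaction menu widget bound to the given minion.
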(event EventBeginPlay
  (bind _returnvalue (UserInterface|CreateWidget "/Game/Blueprints/UI/IngameUI.IngameUI_C" self))
  (bind _output_get (Variables|Default|SetIngameUI_Ref _returnvalue))
  (UserInterface|Viewport|AddtoViewport _output_get 0))

(event EventOnInteract
  (params (Minion :type HOTRELOADED%20Minion%206%20Object%20Reference))
  (bind _returnvalue (UserInterface|CreateWidget "/Game/Blueprints/UI/WB_InteractionMenu.WB_InteractionMenu_C" self Minion))
  (UserInterface|Viewport|AddtoViewport _returnvalue 0))

(event EventOnMinionEnter
  (Default|ShowHint (Variables|Default|GetIngameUI_ref) true))

(event EventOnMinionLeft
  (Default|ShowHint (Variables|Default|GetIngameUI_ref) false))

(fn ConstructionScript)